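; BP_Tile is a base world tile that procedurally grows the map around the top-down player character and removes distant tiles.
; When the player enters its detection collision, it checks four side spawnpoints for overlapping tiles.
; Each free side spawns a random tile class from that side's entry in the PossibleAdjacentTiles map.
; Tick destroys the tile beyond DespawnDistance from the player; a work-in-progress spawnpoint overlap filter is left unconnected.
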(event `self.ReceiveBeginPlay`
  (bind _spawnpoints (`self.Spawnpoints`))
  ;[0 0 1] On begin play, the player is set and the spawnpoints are added to the array.
  (bind _returnvalue (`GameplayStatics.GetActorOfClass` "/Game/TopDown/Blueprints/BP_TopDownCharacter.BP_TopDownCharacter_C"))
  (bind _output_get (set `self.PlayerRef` _returnvalue))
  (`/Engine/EditorBlueprintResources/StandardMacros.IsValid` _output_get
    (:`Is Valid`
      (`KismetArrayLibrary.Array_Add` _spawnpoints (`self.Spawn_Top`))
      (`KismetArrayLibrary.Array_Add` _spawnpoints (`self.Spawn_Right`))
      (`KismetArrayLibrary.Array_Add` _spawnpoints (`self.Spawn_Bottom`))
      (`KismetArrayLibrary.Array_Add` _spawnpoints (`self.Spawn_Left`)))
    (:`Is Not Valid`
      (`KismetSystemLibrary.PrintString` "Warning! Player not set in BP_Tile!" true true (struct :`R` 1.0 :`G` 1.0 :`A` 1.0) 25.0))))

(event `self.Collision_PlayerDetection.OnComponentBeginOverlap`
  (params (OverlappedComponent :type "PrimitiveComponent Object Reference") (OtherActor :type "Actor Object Reference") (OtherComp :type "PrimitiveComponent Object Reference") (OtherBodyIndex :type Integer) (bFromSweep :type Boolean) (SweepResult :type "HitResult Structure (by ref)"))
  ;[0 0 1] When the player starts overlapping a tile, the ones surrounding it are spawned in.
  (if (== OtherActor (`self.PlayerRef`))
    (`self.SpawnAdjacentTiles`)))

(event `self.ReceiveTick`
  (params (DeltaSeconds :type "Float (single-precision)"))
  ;[0 0 1] Checks if the player is further from a tile than the despawn distance and destroys the tile. Tick interval increased to 3 seconds.
  (if (>= (`self.GetDistanceTo` (`self.PlayerRef`) self) (`self.DespawnDistance`))
    (`self.K2_DestroyActor`)))

(fn `SpawnAdjacentTiles`
  (locals (OverlappedComponent :type "ActorComponent Object Reference") (Spawnpoint :type "StaticMeshComponent Object Reference") (SpawnpointIndex :type Integer))
  (bind _value (`BlueprintMapLibrary.Map_Find` (`self.PossibleAdjacentTiles`) (select `int` (`local.SpawnpointIndex`) :`0` (enumliteral `/Game/Features/TileSpawner/Enums/E_TileSides` "NewEnumerator0") :`1` (enumliteral `/Game/Features/TileSpawner/Enums/E_TileSides` "NewEnumerator1") :`2` (enumliteral `/Game/Features/TileSpawner/Enums/E_TileSides` "NewEnumerator2") :`3` (enumliteral `/Game/Features/TileSpawner/Enums/E_TileSides` "NewEnumerator3"))))
  ;[0 0 1] Spawns tiles on the spawnpoints that aren't colliding with anything, with the exception of another spawnpoint.
  ;;[0 0 0] Loops through all the spawnpoints of a tile.
  (for (_array_element _array_index) (`self.Spawnpoints`)
    (set `local.Spawnpoint` _array_element)
    (set `local.SpawnpointIndex` _array_index)
    ;;[0 0 0] Check if spawnpoint isn't overlapping with any tile blueprints.
    (if (`KismetArrayLibrary.Array_IsEmpty` (`PrimitiveComponent.GetOverlappingActors` (`local.Spawnpoint`) "BP_Tile_C"))
      ;;[0 0 0] If not, a new tile is spawned according to the list of possible adjacent tiles.
      (`|SpawnActorFromClass` (`|GetArrayItem` (break `/Game/Features/TileSpawner/Structs/S_PossibleAdjacentTiles` _value) (`KismetMathLibrary.RandomInteger` (- (`KismetArrayLibrary.Array_Length` (break `/Game/Features/TileSpawner/Structs/S_PossibleAdjacentTiles` _value)) 1))) (`KismetMathLibrary.MakeTransform` (`SceneComponent.K2_GetComponentLocation` (`local.Spawnpoint`))) "AlwaysSpawn" "OverrideRootScale" null null)))
  (return))

(fn `UserConstructionScript`)